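; Interactable switch actor, named as a four-color switch, that checks a player's answer entered through a UI widget.
; Overlapping its box shows prompt text and enables input, so releasing F opens the widget created at BeginPlay with mouse cursor and UI-only input.
; The widget's bound events return the input, which is compared to CorrectAnswer to fire correct or wrong dispatchers, and clear the shown flag on hide.
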(event OnComponentBeginOverlap(boxCollision)
  (params (OverlappedComponent :type Primitive%20Component%20Object%20Reference) (OtherActor :type Actor%20Object%20Reference) (OtherComp :type Primitive%20Component%20Object%20Reference) (OtherBodyIndex :type Integer) (bFromSweep :type Boolean) (SweepResult :type Hit%20Result%20Structure%20%28by%20ref%29))
  (Rendering|SetVisibility (Variables|Default|GetTextRender) true false)
  (Input|EnableInput (Game|GetPlayerController 0)))

(event OnComponentEndOverlap(boxCollision)
  (params (OverlappedComponent :type Primitive%20Component%20Object%20Reference) (OtherActor :type Actor%20Object%20Reference) (OtherComp :type Primitive%20Component%20Object%20Reference) (OtherBodyIndex :type Integer))
  (Rendering|SetVisibility (Variables|Default|GetTextRender) false false)
  (Input|DisableInput (Game|GetPlayerController 0)))

(event Custom|onCorrect
  (params (userInput :type Integer))
  (if (== userInput (Variables|Default|GetcorrectAnswer))
    (Default|CallOnAnswerCorrect userInput)
    (else
      (Default|CallOnAnswerWrong userInput))))

(event Custom|onHideUi
  (Variables|Default|SetisShowUi false))

(event EventBeginPlay
  (Utilities|FlowControl|Sequence
    (:then_0
      (bind _returnvalue (UserInterface|CreateWidget "/Game/Maps/Level2/bp_switch_ui.bp_switch_ui_C"))
      (Variables|Default|SetswitchUi _returnvalue))
    (:then_1
      (EventDispatchers|BindEventtoOnCorrect (Variables|Default|GetswitchUi) (delegate Custom|onCorrect)))
    (:then_2
      (EventDispatchers|BindEventtoOnHideUi (Variables|Default|GetswitchUi) (delegate Custom|onHideUi)))))

(event Collision|EventActorBeginOverlap
  (params (OtherActor :type Actor%20Object%20Reference)))

(event EventTick
  (params (DeltaSeconds :type Float%20%28single-precision%29)))

(event Input|KeyboardEvents|F
  (params (Key :type Key%20Structure :default "None"))
  (bind _returnvalue (Game|GetPlayerController 0))
  (:Released
    (if (not (Variables|Default|GetisShowUi))
      (UserInterface|Viewport|AddtoViewport (Variables|Default|GetswitchUi) 0)
      (Variables|Default|SetisShowUi true)
      (Variables|/Script/Engine.PlayerController|SetbShowMouseCursor _returnvalue true)
      (Input|SetInputModeUIOnly _returnvalue 0 "DoNotLock"))))

(fn ConstructionScript)